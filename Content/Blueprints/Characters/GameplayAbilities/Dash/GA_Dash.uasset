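; Gameplay ability that dashes the owning character forward, damaging, pushing and stunning characters it hits.
; On activation it commits, zeroes ground friction, applies a forward velocity impulse, sets pawn collision to overlap and plays the dash montage.
; A gameplay event wait applies the damage effect to each reported target and shoves it away from the dasher.
; Any montage exit restores friction and blocking collision, starts the UI cooldown and ends the ability.
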(event `self.K2_ActivateAbility`
  (`self.K2_CommitAbility`)
  (bind _asbp_character_base (cast `/Game/Blueprints/Characters/BP_CharacterBase` (`self.GetOwningActorFromActorInfo`)))
  (bind _charactermovement (`Character.CharacterMovement` _asbp_character_base))
  (set `self.OriginalGround Friction` (`CharacterMovementComponent.GroundFriction` _charactermovement))
  (set `CharacterMovementComponent.GroundFriction` 0.0 _charactermovement)
  (`CharacterMovementComponent.AddImpulse` _charactermovement (* (`Actor.GetActorForwardVector` _asbp_character_base) 2000.0) true)
  (bind _character (`self.GetPlayerCharacterAndController`))
  (`/Game/Blueprints/Characters/BP_CharacterBase.SetCollisionToPawn` _character "ECR_Overlap")
  (`AbilityTask_PlayMontageAndWait.CreatePlayMontageAndWaitProxy` "None" "/Game/Blueprints/Characters/Animation/AM_Shinbi_Dash.AM_Shinbi_Dash"
    (:`then`
      (bind (_asynctaskproxy _payload) (`AbilityTask_WaitGameplayEvent.WaitGameplayEvent` (struct :`TagName` "skill.dash.dealDamage") null)
        (:`EventReceived`
          (bind (_eventtag _instigator _target) (break `GameplayEventData` _payload))
          (`self.BP_ApplyGameplayEffectToTarget` (`AbilitySystemBlueprintLibrary.AbilityTargetDataFromActor` _target) "/Game/Blueprints/Characters/GameplayAbilities/Dash/GE_Dash_Damage.GE_Dash_Damage_C")
          (bind _asbp_character_base_2 (cast `/Game/Blueprints/Characters/BP_CharacterBase` _target))
          (`/Game/Blueprints/Characters/BP_CharacterBase.PushCharacter` _asbp_character_base_2 (`KismetMathLibrary.Normal` (- (`Actor.K2_GetActorLocation` _asbp_character_base_2) (`Actor.K2_GetActorLocation` (`self.GetOwningActorFromActorInfo`)))) 4000.0 5.0))))
    (:`OnCompleted`
      (set `CharacterMovementComponent.GroundFriction` (`self.OriginalGround Friction`) _charactermovement :!label _label)
      (bind _character_2 (`self.GetPlayerCharacterAndController`))
      (`/Game/Blueprints/Characters/BP_CharacterBase.SetCollisionToPawn` _character_2 "ECR_Block")
      (`self.DoUICooldown`)
      (`self.K2_EndAbility`))
    (:`OnBlendOut`
      (goto _label))
    (:`OnInterrupted`
      (goto _label))
    (:`OnCancelled`
      (goto _label))))