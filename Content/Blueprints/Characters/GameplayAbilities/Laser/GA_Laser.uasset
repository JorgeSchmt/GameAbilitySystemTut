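; Gameplay ability that fires a laser, damaging, pushing and briefly stunning characters it hits.
; After commit and UI cooldown, it plays a casting montage, attaches a spawned BP_Laser to the mesh socket and enables camera-controlled rotation.
; Damage gameplay events apply GE_Laser_Damage and knock targets away from the beam's end detector, ending the ability once cost runs out.
; Ending removes the cost-draining effect, destroys the laser and restores rotation.
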(event `self.K2_ActivateAbility`
  (`self.K2_CommitAbility`)
  (`self.DoUICooldown`)
  (`AbilityTask_PlayMontageAndWait.CreatePlayMontageAndWaitProxy` "None" "/Game/Blueprints/Characters/Animation/AM_Laser_Casting.AM_Laser_Casting" 1.0 "None"
    (:`then`
      (`KismetSystemLibrary.Delay` 0.3)
      (bind _character (`self.GetPlayerCharacterAndController`))
      (bind (_asynctaskproxy _spawnedactor) (`AbilityTask_SpawnActor.SpawnActor` (struct) "/Game/Blueprints/Characters/GameplayAbilities/Laser/BP_Laser.BP_Laser_C" _character)
        (:`then`
          (bind _output_get (set `self.LaserActor` _spawnedactor))
          (`Actor.K2_AttachToComponent` _output_get (`Character.Mesh` _character) "Laser" "SnapToTarget" "SnapToTarget" "SnapToTarget" true)
          (`/Game/Blueprints/Characters/BP_CharacterBase.MakeCameraControlRotation` _character true)
          (bind (_asynctaskproxy_2 _payload) (`AbilityTask_WaitGameplayEvent.WaitGameplayEvent` (struct :`TagName` "skill.laser.dealDamage") null)
            (:`EventReceived`
              (bind _can (`self.IsCostStillAvailblae`))
              (if _can
                (bind (_eventtag _instigator _target _optionalobject _optionalobject2 _contexthandle _instigatortags _targettags _eventmagnitude _targetdata) (break `GameplayEventData` _payload))
                (`self.BP_ApplyGameplayEffectToTarget` _targetdata "/Game/Blueprints/Characters/GameplayAbilities/Laser/GE_Laser_Damage.GE_Laser_Damage_C")
                (for _array_element (`AbilitySystemBlueprintLibrary.GetActorsFromTargetData` _targetdata)
                  (bind _asbp_character_base (cast `/Game/Blueprints/Characters/BP_CharacterBase` _array_element))
                  (`/Game/Blueprints/Characters/BP_CharacterBase.PushCharacter` _asbp_character_base (`KismetMathLibrary.Normal` (- (`Actor.K2_GetActorLocation` _array_element) (`SceneComponent.K2_GetComponentLocation` (`/Game/Blueprints/Characters/GameplayAbilities/Laser/BP_Laser.LaserEndDetector` (cast `/Game/Blueprints/Characters/GameplayAbilities/Laser/BP_Laser` (`self.LaserActor`) :!pure true))))) 500.0 0.3))
                (else
                  (`self.K2_EndAbility`))))))))))

(event `self.K2_OnEndAbility`
  (params (bWasCancelled :type Boolean))
  (`self.BP_RemoveGameplayEffectFromOwnerWithAssetTags` (struct :`GameplayTags` (struct :`(TagName` "skill.laser.drainingCost"))))
  (`Actor.K2_DestroyActor` (`self.LaserActor`))
  (bind _character (`self.GetPlayerCharacterAndController`))
  (`/Game/Blueprints/Characters/BP_CharacterBase.MakeCameraControlRotation` _character false))