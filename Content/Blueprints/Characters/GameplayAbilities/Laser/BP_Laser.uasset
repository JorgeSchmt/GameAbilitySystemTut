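; Laser beam actor for a gameplay ability that periodically signals damage on hostile characters it touches.
; LaserEndDetector overlaps maintain a list of characters hostile to the instigator.
; A looping timer sends that list to the instigator as target data in a Skill.laser.dealDamage gameplay event, even when empty.
; Each tick, the beam AnimBP's end-bone offset follows the detector's distance from the actor, resizing the mesh.
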(event `self.ReceiveBeginPlay`
  (set `self.BeamOrigLen` (`KismetMathLibrary.VSize` (- (`SceneComponent.GetSocketLocation` (`self.LaserMesh`) "end") (`self.K2_GetActorLocation`))))
  ;[1 1 1] Send damage effects every .3 seconds
  (`KismetSystemLibrary.K2_SetTimerDelegate` (delegate `SendDealDamageEvent`) 0.3 true))

(event `SendDealDamageEvent`
  (bind _overlappingactors (`self.OverlappingActors`))
  ;[1 1 1] Send damage effects every .3 seconds
  (if (> (`KismetArrayLibrary.Array_Length` _overlappingactors) 0)
    _
    (else
      _))
  (`AbilitySystemBlueprintLibrary.SendGameplayEventToActor` (`self.GetInstigator`) (struct :`TagName` "skill.laser.dealDamage") (make `GameplayEventData` (struct) null null null null (struct) (struct) (struct) 0.0 (`AbilitySystemBlueprintLibrary.AbilityTargetDataFromActorArray` _overlappingactors))))

(event `self.ReceiveTick`
  (params (DeltaSeconds :type "Float (single-precision)"))
  (bind _asanim_bp_laser_beam (cast `/Game/Blueprints/Characters/GameplayAbilities/Laser/LaserAssets/AnimBP_LaserBeam` (`SkeletalMeshComponent.GetAnimInstance` (`self.LaserMesh`))))
  (set `/Game/Blueprints/Characters/GameplayAbilities/Laser/LaserAssets/AnimBP_LaserBeam.EndOfBoneOffset` (`KismetMathLibrary.MakeVector` (`KismetMathLibrary.VSize` (- (`SceneComponent.K2_GetComponentLocation` (`self.LaserEndDetector`)) (`self.K2_GetActorLocation`)))) _asanim_bp_laser_beam))

(event `self.LaserEndDetector.OnComponentBeginOverlap`
  (params (OverlappedComponent :type "PrimitiveComponent Object Reference") (OtherActor :type "Actor Object Reference") (OtherComp :type "PrimitiveComponent Object Reference") (OtherBodyIndex :type Integer) (bFromSweep :type Boolean) (SweepResult :type "HitResult Structure (by ref)"))
  (bind _asbp_character_base (cast `/Game/Blueprints/Characters/BP_CharacterBase` OtherActor))
  (bind _asbp_character_base_2 (cast `/Game/Blueprints/Characters/BP_CharacterBase` (`self.GetInstigator`)))
  (if (`CharacterBase.IsOtherHostile` _asbp_character_base_2 _asbp_character_base)
    (`KismetArrayLibrary.Array_AddUnique` (`self.OverlappingActors`) _asbp_character_base)))

(event `self.LaserEndDetector.OnComponentEndOverlap`
  (params (OverlappedComponent :type "PrimitiveComponent Object Reference") (OtherActor :type "Actor Object Reference") (OtherComp :type "PrimitiveComponent Object Reference") (OtherBodyIndex :type Integer))
  (bind _asbp_character_base (cast `/Game/Blueprints/Characters/BP_CharacterBase` OtherActor))
  (`KismetArrayLibrary.Array_RemoveItem` (`self.OverlappingActors`) _asbp_character_base))

(fn `UserConstructionScript`)