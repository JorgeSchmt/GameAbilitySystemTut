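; BP_CharacterBase is a base character Blueprint that uses the Gameplay Ability System for melee, dash and health regen.
; It acquires the three abilities on BeginPlay and exposes events to activate each.
; Sword and capsule overlaps with hostile characters send tagged gameplay events to self, carrying the target for melee or dash damage.
; It also handles montage-then-destroy death, pushes with briefly zeroed ground friction, and setting capsule response to pawns.
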(event `self.ReceiveBeginPlay`
  (`self.AcquireAbility` "/Game/Blueprints/Characters/GameplayAbilities/Melee/GA_Melee.GA_Melee_C")
  (`self.AcquireAbility` "/Game/Blueprints/Characters/GameplayAbilities/HealthRegen/GA_HealthRegen.GA_HealthRegen_C")
  (`self.AcquireAbility` "/Game/Blueprints/Characters/GameplayAbilities/Dash/GA_Dash.GA_Dash_C"))

(event `TryHealthRegen`
  (`AbilitySystemComponent.TryActivateAbilityByClass` (`self.AbilitySystemComp`) "/Game/Blueprints/Characters/GameplayAbilities/HealthRegen/GA_HealthRegen.GA_HealthRegen_C" true))

(event `MeleeAttack`
  (`AbilitySystemComponent.TryActivateAbilityByClass` (`self.AbilitySystemComp`) "/Game/Blueprints/Characters/GameplayAbilities/Melee/GA_Melee.GA_Melee_C" true))

(event `TryDashAbility`
  (`AbilitySystemComponent.TryActivateAbilityByClass` (`self.AbilitySystemComp`) "/Game/Blueprints/Characters/GameplayAbilities/Dash/GA_Dash.GA_Dash_C" true))

(event `self.SwordCollider.OnComponentBeginOverlap`
  (params (OverlappedComponent :type "PrimitiveComponent Object Reference") (OtherActor :type "Actor Object Reference") (OtherComp :type "PrimitiveComponent Object Reference") (OtherBodyIndex :type Integer) (bFromSweep :type Boolean) (SweepResult :type "HitResult Structure (by ref)"))
  (if (!= OtherActor self)
    (bind _asbp_character_base (cast `/Game/Blueprints/Characters/BP_CharacterBase` OtherActor))
    (if (`self.IsOtherHostile` _asbp_character_base self)
      (`AbilitySystemBlueprintLibrary.SendGameplayEventToActor` self (struct :`TagName` "skill.melee.dealdamage") (make `GameplayEventData` (struct) null OtherActor)))))

(event `self.BP_Die`
  (bind _returnvalue (`self.PlayAnimMontage` "/Game/Blueprints/Characters/Animation/AM_DieShinbi.AM_DieShinbi"))
  (`KismetSystemLibrary.Delay` _returnvalue)
  (`self.K2_DestroyActor`))

(event `self.CapsuleComponent.OnComponentBeginOverlap`
  (params (OverlappedComponent :type "PrimitiveComponent Object Reference") (OtherActor :type "Actor Object Reference") (OtherComp :type "PrimitiveComponent Object Reference") (OtherBodyIndex :type Integer) (bFromSweep :type Boolean) (SweepResult :type "HitResult Structure (by ref)"))
  (bind _asbp_character_base (cast `/Game/Blueprints/Characters/BP_CharacterBase` OtherActor))
  (if (`self.IsOtherHostile` _asbp_character_base self)
    (`AbilitySystemBlueprintLibrary.SendGameplayEventToActor` self (struct :`TagName` "skill.dash.dealDamage") (make `GameplayEventData` (struct) self OtherActor))))

(event `PushCharacter`
  (params (ImpulseDirection :type "Vector Structure") (PushStrength :type "Float (double-precision)"))
  (bind _charactermovement (`self.CharacterMovement`))
  (set `self.Ground FrictionOriginal` (`CharacterMovementComponent.GroundFriction` _charactermovement))
  (set `CharacterMovementComponent.GroundFriction` 0.0 _charactermovement)
  (`CharacterMovementComponent.AddImpulse` _charactermovement (* ImpulseDirection PushStrength) true)
  (`KismetSystemLibrary.Delay` 0.3)
  (set `CharacterMovementComponent.GroundFriction` (`self.Ground FrictionOriginal`) _charactermovement))

(fn `SetCollisionToPawn`
  (params (NewResponse :type "ECollisionResponse Enum" :default "ECR_Ignore"))
  (`PrimitiveComponent.SetCollisionResponseToChannel` (`self.CapsuleComponent`) "ECC_Pawn" NewResponse))

(fn `UserConstructionScript`)